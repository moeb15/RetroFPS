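; BP_ManaPickup is a RetroFPS mana pickup shown as a flipbook that floats up and down.
; On sphere overlap it passes the other actor to ApplyEffectToTarget, whose logic is not defined in this graph.
; Each Tick, FloatingEffect adds OscillationSpeed times the sine of elapsed time to the flipbook's current relative Z, so the bob accumulates per frame and depends on frame rate.
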(event OnComponentBeginOverlap(Sphere)
  (params (OverlappedComponent :type Primitive%20Component%20Object%20Reference) (OtherActor :type Actor%20Object%20Reference) (OtherComp :type Primitive%20Component%20Object%20Reference) (OtherBodyIndex :type Integer) (bFromSweep :type Boolean) (SweepResult :type Hit%20Result%20Structure%20%28by%20ref%29))
  (Class|PickupActor|ApplyEffecttoTarget OtherActor))

(event EventBeginPlay)

(event Collision|EventActorBeginOverlap
  (params (OtherActor :type Actor%20Object%20Reference)))

(event EventTick
  (params (DeltaSeconds :type Float%20%28single-precision%29))
  (CallFunction|FloatingEffect DeltaSeconds))

(fn ConstructionScript)

(fn FloatingEffect
  (params (DeltaTime :type Float%20%28double-precision%29))
  (bind _pickupflipbook (Variables|Default|GetPickupFlipbook))
  (bind _relativelocation (Variables|/Script/Engine.SceneComponent|GetRelativeLocation _pickupflipbook))
  (bind (_x _y _z) (Math|Vector|BreakVector _relativelocation))
  (bind _output_get (Variables|Default|SetElapsed%20Time (+ (Variables|Default|GetElapsed%20Time) DeltaTime)))
  (Transformation|SetRelativeLocation (Variables|Default|GetPickupFlipbook) (Math|Vector|MakeVector _x _y (+ (* (LocalVariables|GetOscillation%20Speed) (Math|Trig|Sin(Radians) _output_get)) _z)) false false))