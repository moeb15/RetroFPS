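; Pistol weapon Blueprint for the retro FPS, handling the bob and draw animations of its flipbook sprite.
; WeaponBob plays the WeaponMovement sequence while moving, otherwise stops it and interpolates the flipbook back toward a fixed rest position.
; WeaponDraw plays a separate draw sequence.
; It contains no firing logic, and its BeginPlay, overlap and Tick events are unused.
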(event EventBeginPlay)

(event Collision|EventActorBeginOverlap
  (params (OtherActor :type Actor%20Object%20Reference)))

(event EventTick
  (params (DeltaSeconds :type Float%20%28single-precision%29)))

(event EventWeaponBob
  (params (IsMoving :type Boolean) (DeltaTime :type Float%20%28single-precision%29))
  (bind _weapon_movement (Variables|Default|GetWeapon%20Movement))
  (bind _weaponflipbook (Variables|Default|GetWeaponFlipbook))
  (bind _sequenceplayer (Variables|/Script/ActorSequence.ActorSequenceComponent|GetSequencePlayer _weapon_movement))
  (if IsMoving
    (Sequencer|Player|Play _sequenceplayer :!class /Script/MovieScene.MovieSceneSequencePlayer)
    (else
      (Sequencer|Player|Stop _sequenceplayer :!class /Script/MovieScene.MovieSceneSequencePlayer)
      (Transformation|SetRelativeLocation _weaponflipbook (Math|Interpolation|VInterpTo (Variables|/Script/Engine.SceneComponent|GetRelativeLocation _weaponflipbook) "0.000000,100.000000,-50.000000" DeltaTime 5.0) false false))))

(event EventWeaponDraw
  (Class|ActorSequenceComponent|PlaySequence (Variables|Default|GetWeapon%20Draw)))

(fn ConstructionScript)